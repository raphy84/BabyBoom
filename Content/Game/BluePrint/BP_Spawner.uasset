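; BP_Spawner pre-places a hidden, non-colliding child actor and reveals it on a game mode spawn request.
; Construction sets the child class; only for a BP_Ennemie child does it pass the ID and build the "Door"-prefixed SpawnID.
; A matching RequestSpawn plays Niagara, then briefly delays before enabling visibility and collision.
; Tick pins the child to the spawner's transform while collision is off.
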(event Custom|RequestSpawn
  (params (ID :type String))
  (bind _childactor (Variables|Default|GetChildActor))
  (bind _childactor_2 (Variables|/Script/Engine.ChildActorComponent|GetChildActor _childactor))
  (if (Utilities|Enum|Equal(Enum) ID (Variables|Default|GetSpawnID))
    (Components|Activation|Activate (Variables|Default|GetNiagara) false)
    (Utilities|FlowControl|Delay 0.2)
    (Rendering|SetActorHiddenInGame _childactor_2 false)
    (Collision|SetActorEnableCollision _childactor_2 true)))

(event EventBeginPlay
  (bind _asbp_first_person_game_mode (Utilities|Casting|CastToBP_FirstPersonGameMode (Game|GetGameMode)))
  (EventDispatchers|BindEventtoRequestSpawn _asbp_first_person_game_mode (delegate Custom|RequestSpawn)))

(event EventTick
  (params (DeltaSeconds :type Float%20%28single-precision%29))
  (bind _childactor (Variables|Default|GetChildActor))
  (bind _childactor_2 (Variables|/Script/Engine.ChildActorComponent|GetChildActor _childactor))
  (if (not (Collision|GetActorEnableCollision _childactor_2))
    (Transformation|SetActorTransform _childactor_2 (Transformation|GetActorTransform))))

(fn ConstructionScript
  (CallFunction|NewFunction))

(fn NewFunction
  (bind _childactor (Variables|Default|GetChildActor))
  (bind _id (Variables|Default|GetID))
  (bind _childactor_2 (Variables|/Script/Engine.ChildActorComponent|GetChildActor _childactor))
  (ChildActorComponent|SetChildActorClass (Variables|Default|GetChildActor) (Variables|Default|GetClass))
  (Rendering|SetActorHiddenInGame _childactor_2 true)
  (Collision|SetActorEnableCollision _childactor_2 false)
  (bind _asbp_ennemie (Utilities|Casting|CastToBP_Ennemie _childactor_2))
  (bind _output_get (Variables|Default|SetIfEnnemy _asbp_ennemie))
  (Variables|/Game/Game/BluePrint/Ennemie/BP_Ennemie.BP_Ennemie_C|SetEnnemiID _output_get _id)
  (Variables|Default|SetSpawnID (Utilities|String|Append "Door" (Utilities|String|ToString(Integer) _id))))