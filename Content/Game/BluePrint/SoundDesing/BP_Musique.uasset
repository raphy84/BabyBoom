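; BP_Musique is a music player actor that plays a selectable track, optionally starting on BeginPlay.
; The construction script assigns the chosen sound to the audio component.
; LaucheMusique starts playback with a timeline-driven volume fade, while StopMusique reverses a second timeline to fade and then stop.
; Tick matches the music pitch to global time dilation, so the track follows changes in game speed.
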(event Custom|StopMusique
  (bind _volume (Timeline|Timeline_0 Reverse)
    (:Update
      (Audio|Components|Audio|SetVolumeMultiplier (Variables|Default|GetMusique) _volume :!class /Script/Engine.AudioComponent))
    (:Finished
      (Audio|Components|Audio|Stop (Variables|Default|GetMusique)))))

(event Custom|LaucheMusique
  (bind _musique (Variables|Default|GetMusique))
  (Audio|Components|Audio|Play _musique 0.0)
  (bind _volume (Timeline|Timeline PlayFromStart)
    (:Update
      (Audio|Components|Audio|SetVolumeMultiplier _musique _volume :!class /Script/Engine.AudioComponent))))

(event EventBeginPlay
  (bind _musique (Variables|Default|GetMusique))
  (if (Variables|Default|GetStart)
    (Audio|Components|Audio|Play _musique 0.0)
    (bind _volume (Timeline|Timeline PlayFromStart)
      (:Update
        (Audio|Components|Audio|SetVolumeMultiplier _musique _volume :!class /Script/Engine.AudioComponent)))))

(event EventTick
  (params (DeltaSeconds :type Float%20%28single-precision%29))
  (Audio|Components|Audio|SetPitchMultiplier (Variables|Default|GetMusique) (Class|GameplayStatics|GetGlobalTimeDilation)))

(fn ConstructionScript
  (Audio|Components|Audio|SetSound (Variables|Default|GetMusique) (Variables|Default|GetMusiqueSelect)))