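; BP_Claymore is a laser tripwire trap that explodes into shrapnel when a damageable actor crosses one of its beams.
; Every tick, three line traces run from a shared laser origin to left, middle and right arrow components, checking hits for BPI_Damageble.
; A hit triggers a one-time detonation with sound and grenade FX, spawning BP_Chrapnel along an array of arrow transforms before destroying itself after a short delay.
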(event Custom|DestroyClaymore
  (bind _returnvalue (Transformation|GetActorLocation))
  (Utilities|FlowControl|DoOnce false
    (:Completed
      (Audio|PlaySoundatLocation "/Game/Game/SoundDesign/Sound/Ennemie/SC_Clemort.SC_Clemort" _returnvalue "0, 0, 0" 1.0 (Class|GameplayStatics|GetGlobalTimeDilation) 0.0 0 0 0 0)
      (Niagara|SpawnSystematLocation "/Game/Game/BluePrint/Ennemie/Projectil/FX_GRENADE.FX_GRENADE" _returnvalue)
      (for _array_element (Variables|Default|GetArray)
        (Game|SpawnActorfromClass "/Game/Game/BluePrint/Ennemie/Projectil/BP_Chrapnel.BP_Chrapnel_C" (Math|Transform|MakeTransform (Transformation|GetWorldLocation _array_element) (Transformation|GetWorldRotation _array_element) "1.000000,1.000000,1.000000") "AlwaysSpawn" "MultiplyWithRoot" 0 0))
      (Utilities|FlowControl|Delay 0.2)
      (Actor|DestroyActor))))

(event EventBeginPlay
  (Variables|Default|SetArray (Utilities|Array|MakeArray (Variables|Default|GetArrow13) (Variables|Default|GetArrow1) (Variables|Default|GetArrow2) (Variables|Default|GetArrow4) (Variables|Default|GetArrow) (Variables|Default|GetArrow11) (Variables|Default|GetArrow12) (Variables|Default|GetArrow3) (Variables|Default|GetArrow10) (Variables|Default|GetArrow6) (Variables|Default|GetArrow7) (Variables|Default|GetArrow5) (Variables|Default|GetArrow8) (Variables|Default|GetArrow9))))

(event Collision|EventActorBeginOverlap
  (params (OtherActor :type Actor%20Object%20Reference)))

(event EventTick
  (params (DeltaSeconds :type Float%20%28single-precision%29))
  (bind _départlaser1 (Variables|Default|GetDépartLaser1))
  (bind _portéelaser (Variables|Default|GetPortéeLaser))
  (CallFunction|RightLine _départlaser1 _portéelaser)
  (CallFunction|LeftLine _départlaser1 _portéelaser)
  (CallFunction|MiddleLine _départlaser1 _portéelaser))

(fn ConstructionScript)

(fn RightLine
  (params (PointDepart :type Scene%20Component%20Object%20Reference) (PortéeLaser :type Float%20%28double-precision%29))
  (Utilities|IsValid PointDepart
    (:Is%20Valid
      (bind _outhit (Class|KismetSystemLibrary|LineTraceSinglebyProfile (Transformation|GetWorldLocation PointDepart) (Transformation|GetWorldLocation (Variables|Default|GetArrow15)) "Pawn" false 0 "None" true))
      (if (Utilities|DoesObjectImplementInterface (.HitActor (Collision|BreakHitResult _outhit)) "/Game/Game/Interface/BPI_Damageble.BPI_Damageble_C")
        (CallFunction|DestroyClaymore)))))

(fn LeftLine
  (params (PointDepart :type Scene%20Component%20Object%20Reference) (PortéeLaser :type Float%20%28double-precision%29))
  (Utilities|IsValid PointDepart
    (:Is%20Valid
      (bind _outhit (Class|KismetSystemLibrary|LineTraceSinglebyProfile (Transformation|GetWorldLocation PointDepart) (Transformation|GetWorldLocation (Variables|Default|GetArrow14)) "Pawn" false 0 "None" true))
      (if (Utilities|DoesObjectImplementInterface (.HitActor (Collision|BreakHitResult _outhit)) "/Game/Game/Interface/BPI_Damageble.BPI_Damageble_C")
        (CallFunction|DestroyClaymore)))))

(fn MiddleLine
  (params (PointDepart :type Scene%20Component%20Object%20Reference) (PortéeLaser :type Float%20%28double-precision%29))
  (Utilities|IsValid PointDepart
    (:Is%20Valid
      (bind _outhit (Class|KismetSystemLibrary|LineTraceSinglebyProfile (Transformation|GetWorldLocation PointDepart) (Transformation|GetWorldLocation (Variables|Default|GetArrow16)) "Pawn" false 0 "None" true))
      (if (Utilities|DoesObjectImplementInterface (.HitActor (Collision|BreakHitResult _outhit)) "/Game/Game/Interface/BPI_Damageble.BPI_Damageble_C")
        (CallFunction|DestroyClaymore)))))