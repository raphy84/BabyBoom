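; BP_Ennemie is an armed enemy character that, once activated, chases and shoots the player.
; Each tick, blocked sight triggers AI movement toward the player; clear sight leads to random movement near TraceTypeQuery4 hits, otherwise stop, turn and fire BP_Balle.
; Damage comes through TakeDamage, also triggered by fast physics props.
; Death ragdolls the mesh, optionally after a launch, and removes it from its ID-matched door's enemy list.
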(event OnComponentBeginOverlap(CapsuleComponent)
  (params (OverlappedComponent :type Primitive%20Component%20Object%20Reference) (OtherActor :type Actor%20Object%20Reference) (OtherComp :type Primitive%20Component%20Object%20Reference) (OtherBodyIndex :type Integer) (bFromSweep :type Boolean) (SweepResult :type Hit%20Result%20Structure%20%28by%20ref%29))
  (bind _asstatic_mesh_actor (Utilities|Casting|CastToStaticMeshActor OtherActor))
  (if (Physics|IsSimulatingPhysics (Variables|/Script/Engine.StaticMeshActor|GetStaticMeshComponent _asstatic_mesh_actor) "None")
    (if (>= (Math|Vector|VectorLength (Transformation|GetVelocity _asstatic_mesh_actor)) 3e+02)
      (CallFunction|TakeDamage 5 "0, 0, 0"))))

(event EventTakeDamage
  (params (Degat :type Integer) (HitLocation :type Vector :default "0, 0, 0"))
  (Utilities|FlowControl|DoOnce false
    (:Completed
      (bind _output_get (Variables|Default|SetPV (- (Variables|Default|GetPV) Degat)))
      (if (<= _output_get 0)
        (Variables|Default|SetDead true)
        (Audio|PlaySoundatLocation "/Game/Game/SoundDesign/Sound/Ennemie/SC_EnnemieDead.SC_EnnemieDead" (Transformation|GetActorLocation) "0, 0, 0" 1.0 (Class|GameplayStatics|GetGlobalTimeDilation) 0.0 0 0 0 0)
        (if (Utilities|Operators|EqualEqual :A HitLocation)
          (Components|DestroyComponent (Variables|Default|GetCanonFusil))
          (Physics|SetSimulatePhysics (Variables|Character|GetMesh) true)
          (else
            (Character|LaunchCharacter (* HitLocation "500.000000,500.000000,500.000000") false false)
            (Utilities|FlowControl|Delay 0.1)
            (Components|DestroyComponent (Variables|Default|GetCanonFusil))
            (Physics|SetSimulatePhysics (Variables|Character|GetMesh) true)))
        (bind _array_element (Utilities|Array|ForEachLoopwithBreak (Variables|/Game/Game/BluePrint/BP_FirstPersonGameMode.BP_FirstPersonGameMode_C|GetDoorList (Variables|Default|GetAs%20BP%20First%20Person%20Game%20Mode)) :!label _label)
          (:LoopBody
            (if (== (Variables|/Game/Game/BluePrint/LevelDesignTools/BP_Door.BP_Door_C|GetPorteID _array_element) (Variables|Default|GetEnnemiID))
              (goto _label Break)))
          (:Completed
            (Default|RemoveEnnemisfromList _array_element self)))))))

(event EventTick
  (params (DeltaSeconds :type Float%20%28single-precision%29))
  (bind _returnvalue (Transformation|GetActorLocation))
  (bind _canonfusil (Variables|Default|GetCanonFusil))
  (bind _canonfusil_2 (Variables|Default|GetCanonFusil))
  (bind _returnvalue_2 (Transformation|GetWorldLocation _canonfusil_2))
  (if (Variables|Default|GetIsActivate)
    (if (not (Variables|Default|GetDead))
      (bind (_outhit _returnvalue_3) (Collision|SphereTraceByChannel (Transformation|GetWorldLocation (Variables|Default|GetVue)) (Transformation|GetWorldLocation (Variables|/Game/Game/BluePrint/BP_FirstPersonCharacter.BP_FirstPersonCharacter_C|GetTargetEnnemie (Variables|Default|GetAs%20BP%20First%20Person%20Character))) 1e+01 "TraceTypeQuery1" false 0 "None"))
      (if _returnvalue_3
        (if (not (Variables|Default|GetNoMovement))
          (AI|AIMoveTo (Class|PawnMovementComponent|GetPawnOwner (Variables|Character|GetCharacterMovement)) "0, 0, 0" (Game|GetPlayerCharacter 0) 0.0 false
            (:then
              (Variables|Default|SetArme (stale _arme)))))
        (else
          (bind (_outhit_2 _returnvalue_4) (Collision|SphereTraceByChannel _returnvalue _returnvalue 1e+02 "TraceTypeQuery4" false 0 "None" true "(R=1.000000,G=0.000000,B=0.705958,A=1.000000)" "(R=0.000000,G=0.057080,B=1.000000,A=1.000000)"))
          (if _returnvalue_4
            (Utilities|FlowControl|Sequence
              (:then_0
                (Utilities|FlowControl|DoOnce false :!label _label
                  (:Completed
                    (Variables|Default|SetImpact%20Point (Variables|Default|GetImpact%20Point) :!label _label_2)
                    (Variables|Default|SetRandom (Math|Random|RandomFloatinRange -1.0 1.0))
                    (Utilities|FlowControl|Delay 4.0)
                    (if _returnvalue_4
                      (goto _label_2)))))
              (:then_1
                (Pawn|Input|AddMovementInput (.ImpactPoint (Collision|BreakHitResult _outhit_2)) (Variables|Default|GetRandom) false)))
            (else
              (Utilities|FlowControl|Sequence
                (:then_0
                  (Class|NavMovementComponent|StopActiveMovement (Variables|Character|GetCharacterMovement))
                  (Transformation|SetActorRotation (Math|Rotator|MakeRotator 0.0 0.0 (.yaw (Math|Rotator|FindLookatRotation (Transformation|GetActorLocation) (Transformation|GetActorLocation (Game|GetPlayerCharacter 0))))))
                  (Utilities|FlowControl|DoOnce false :!label _label_3
                    (:Completed
                      (Variables|Default|SetNoMovement true)
                      (Variables|Default|SetArme 25.0)
                      (Utilities|FlowControl|Delay 0.5)
                      (Utilities|IsValid (Variables|Default|GetCanonFusil)
                        (:Is%20Valid
                          (Audio|PlaySoundatLocation "/Game/Game/SoundDesign/Sound/Ennemie/SC_TireFusilAssaut.SC_TireFusilAssaut" (Transformation|GetActorLocation) "0, 0, 0" (Math|Random|RandomFloatinRange 0.2 0.75) (Class|GameplayStatics|GetGlobalTimeDilation) 0.0 0 0 0 0)
                          (Niagara|SpawnSystematLocation "/Game/Game/3d/Mesh/Ennemie/FX/FX_WEAPON.FX_WEAPON" (Transformation|GetWorldLocation _canonfusil) (Transformation|GetWorldRotation _canonfusil))
                          (Game|SpawnActorfromClass "/Game/Game/BluePrint/Ennemie/Projectil/BP_Balle.BP_Balle_C" (Math|Transform|MakeTransform _returnvalue_2 (Math|Rotator|FindLookatRotation _returnvalue_2 (Transformation|GetActorLocation (Game|GetPlayerCharacter 0))) "1.000000,1.000000,1.000000") "Undefined" "MultiplyWithRoot" 0 0)
                          (Utilities|FlowControl|Delay 0.5)
                          (Variables|Default|SetNoMovement false)
                          (goto _label_3 Reset))))))
                (:then_1
                  (goto _label Reset))))))))))

(event EventBeginPlay
  (bind _asbp_first_person_character (Utilities|Casting|CastToBP_FirstPersonCharacter (Game|GetPlayerCharacter 0)))
  (Variables|Default|SetAs%20BP%20First%20Person%20Character _asbp_first_person_character)
  (bind _asbp_first_person_game_mode (Utilities|Casting|CastToBP_FirstPersonGameMode (Game|GetGameMode)))
  (Variables|Default|SetAs%20BP%20First%20Person%20Game%20Mode _asbp_first_person_game_mode))

(fn ConstructionScript)