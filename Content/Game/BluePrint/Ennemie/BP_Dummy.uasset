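; BP_Dummy is an enemy training dummy that repeatedly fires training balls.
; After an initial delay on BeginPlay, it spawns a BP_TrainingBalle at the Muzzul component's location and rotation, then launches it with a strong impulse along the muzzle's forward vector.
; A Delay node wired back to the spawn forms an endless firing loop, with no targeting or use of Tick.
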(event EventBeginPlay
  (bind _muzzul (Variables|Default|GetMuzzul))
  (Utilities|FlowControl|Delay 5.0)
  (bind _returnvalue (Game|SpawnActorfromClass "/Game/Game/BluePrint/Ennemie/Projectil/BP_TrainingBalle.BP_TrainingBalle_C" (Math|Transform|MakeTransform (Transformation|GetWorldLocation _muzzul) (Transformation|GetWorldRotation _muzzul) "1.000000,1.000000,1.000000") "Undefined" "MultiplyWithRoot" 0 0 :!label _label))
  (Physics|AddImpulse (Variables|/Script/Engine.StaticMeshActor|GetStaticMeshComponent _returnvalue) (* (Math|Vector|GetForwardVector (Variables|Default|GetMuzzul)) 3e+05) "None" false)
  (Utilities|FlowControl|Delay 3.0)
  (goto _label))

(event Collision|EventActorBeginOverlap
  (params (OtherActor :type Actor%20Object%20Reference)))

(event EventTick
  (params (DeltaSeconds :type Float%20%28single-precision%29)))

(fn ConstructionScript)