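; BP_Chrapnel is a shrapnel projectile that damages actors implementing BPI_Damageble on capsule overlap, ignoring other shrapnel.
; BP_Ennemie targets take more damage and spawn an explosion effect, while non-damageable surfaces get a wall-impact effect.
; Each hit hides the mesh, deactivates it and detaches the Niagara effect before delayed destruction.
; Tick matches sound pitch to time dilation and plays a one-shot sound when a proximity sphere trace hits.
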(event OnComponentBeginOverlap(Capsule)
  (params (OverlappedComponent :type Primitive%20Component%20Object%20Reference) (OtherActor :type Actor%20Object%20Reference) (OtherComp :type Primitive%20Component%20Object%20Reference) (OtherBodyIndex :type Integer) (bFromSweep :type Boolean) (SweepResult :type Hit%20Result%20Structure%20%28by%20ref%29))
  (Utilities|Casting|CastToBP_Chrapnel OtherActor
    (:CastFailed
      (if (not (Variables|Default|GetDeactivate))
        (if (Utilities|DoesObjectImplementInterface OtherActor "/Game/Game/Interface/BPI_Damageble.BPI_Damageble_C")
          (Utilities|Casting|CastToBP_Ennemie OtherActor
            (:then
              (Class|BPIDamageble|TakeDamage(Message) OtherActor 5 (Transformation|GetActorForwardVector))
              (Rendering|SetVisibility (Variables|Default|GetSM_PACK_1_BALLE) false false)
              (Variables|Default|SetDeactivate true)
              (Niagara|SpawnSystematLocation "/Game/Game/BluePrint/Trap/Explosion_TETE.Explosion_TETE" (Transformation|GetActorLocation))
              (Transformation|DetachFromComponent (Variables|Default|GetNiagara) "KeepWorld" "KeepWorld" "KeepWorld" true)
              (Utilities|FlowControl|Delay 1.0)
              (Actor|DestroyActor))
            (:CastFailed
              (Class|BPIDamageble|TakeDamage(Message) OtherActor 3 "0, 0, 0")
              (Rendering|SetVisibility (Variables|Default|GetSM_PACK_1_BALLE) false false)
              (Variables|Default|SetDeactivate true)
              (Transformation|DetachFromComponent (Variables|Default|GetNiagara) "KeepWorld" "KeepWorld" "KeepWorld" true)
              (Utilities|FlowControl|Delay 1.0)
              (Actor|DestroyActor)))
          (else
            (Rendering|SetVisibility (Variables|Default|GetSM_PACK_1_BALLE) false false)
            (Variables|Default|SetDeactivate true)
            (Transformation|DetachFromComponent (Variables|Default|GetNiagara) "KeepWorld" "KeepWorld" "KeepWorld" true)
            (Niagara|SpawnSystematLocation "/Game/Game/BluePrint/Trap/NS_TouchMur.NS_TouchMur" (Transformation|GetActorLocation))
            (Components|DestroyComponent (Variables|Default|GetNiagara1))
            (Utilities|FlowControl|Delay 2.0)
            (Actor|DestroyActor)))))))

(event Custom|CanKill
  (Variables|Default|SetCanKillFrend true))

(event EventBeginPlay
  (Utilities|FlowControl|Delay 5.0)
  (Variables|Default|SetCanKillFrend true))

(event Collision|EventActorBeginOverlap
  (params (OtherActor :type Actor%20Object%20Reference)))

(event EventTick
  (params (DeltaSeconds :type Float%20%28single-precision%29))
  (bind _returnvalue (Transformation|GetActorLocation))
  (if (not (Variables|Default|GetDeactivate))
    (Audio|Components|Audio|SetPitchMultiplier (Variables|Default|GetSoundSpeed) (Class|GameplayStatics|GetGlobalTimeDilation))
    (bind _returnvalue_2 (Collision|SphereTraceByChannel _returnvalue _returnvalue 1.2e+02 "TraceTypeQuery5" false 0 "None"))
    (if _returnvalue_2
      (Utilities|FlowControl|DoOnce false
        (:Completed
          (Audio|Components|Audio|Play (Variables|Default|GetSoundSpeed) 0.0))))))

(fn ConstructionScript)