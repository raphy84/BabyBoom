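; BP_Grenade is an enemy projectile that explodes on a three-second fuse after BeginPlay.
; When the timer fires, it spawns an explosion particle and runs a multi sphere trace on the Pawn profile at its location.
; Hit actors implementing BPI_Damageble receive fixed damage through an interface message.
; DestroyActor sits inside the hit loop, so the grenade is removed only when the trace hits something.
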(event Custom|DestroyGrenade
  (bind _returnvalue (Transformation|GetActorLocation))
  (Effects|SpawnEmitteratLocation "/Game/StarterContent/Particles/P_Explosion.P_Explosion" _returnvalue)
  (bind _outhits (Class|KismetSystemLibrary|SphereTraceMultibyProfile _returnvalue _returnvalue 2e+02 "Pawn" false 0 "None" true))
  (for _array_element _outhits
    (if (Utilities|DoesObjectImplementInterface (.HitActor (Collision|BreakHitResult _array_element)) "/Game/Game/Interface/BPI_Damageble.BPI_Damageble_C")
      (Class|BPIDamageble|TakeDamage(Message) (.HitActor (Collision|BreakHitResult _array_element)) 3 "0, 0, 0"))
    (Actor|DestroyActor)))

(event EventBeginPlay
  (Utilities|Time|SetTimerbyEvent (delegate Custom|DestroyGrenade) 3.0))

(event Collision|EventActorBeginOverlap
  (params (OtherActor :type Actor%20Object%20Reference)))

(event EventTick
  (params (DeltaSeconds :type Float%20%28single-precision%29)))

(fn ConstructionScript)