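; Tutorial sliding double door that opens as the player approaches and seals behind them to start that room's enemy encounter.
; One one-shot trigger opens it, sliding both panels and switching BP_Musique actors to the SC_Lex track.
; Another closes it, requests a game-mode spawn by PorteID and activates enemies with that ID.
; RemoveEnnemisFromList reopens it when the room list empties, though the code filling that list is disconnected.
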(event OnComponentBeginOverlap(CollisionBox)
  (params (OverlappedComponent :type Primitive%20Component%20Object%20Reference) (OtherActor :type Actor%20Object%20Reference) (OtherComp :type Primitive%20Component%20Object%20Reference) (OtherBodyIndex :type Integer) (bFromSweep :type Boolean) (SweepResult :type Hit%20Result%20Structure%20%28by%20ref%29))
  (Utilities|Casting|CastToBP_FirstPersonCharacter OtherActor)
  (if (not (Variables|Default|GetBlockDoor))
    (CallFunction|CloseDoor)
    (Variables|Default|SetBlockDoor true)
    (Audio|PlaySound2D "/Game/Game/SoundDesign/Sound/Ennemie/SC_Hey.SC_Hey" 1.0 1.0 0.7 0 0)
    (Default|CallRequestSpawn (Variables|Default|GetAs%20BP%20First%20Person%20Game%20Mode) (Utilities|String|Append "Door" (Utilities|String|ToString(Integer) (Variables|Default|GetPorteID))))
    (for _array_element (Variables|/Game/Game/BluePrint/BP_FirstPersonGameMode.BP_FirstPersonGameMode_C|GetEnnemiList (Variables|Default|GetAs%20BP%20First%20Person%20Game%20Mode))
      (if (== (Variables|/Game/Game/BluePrint/Ennemie/BP_Ennemie.BP_Ennemie_C|GetEnnemiID _array_element) (Variables|Default|GetPorteID))
        (Variables|/Game/Game/BluePrint/Ennemie/BP_Ennemie.BP_Ennemie_C|SetIsActivate _array_element true)))))

(event OnComponentBeginOverlap(OpenDoorColl)
  (params (OverlappedComponent :type Primitive%20Component%20Object%20Reference) (OtherActor :type Actor%20Object%20Reference) (OtherComp :type Primitive%20Component%20Object%20Reference) (OtherBodyIndex :type Integer) (bFromSweep :type Boolean) (SweepResult :type Hit%20Result%20Structure%20%28by%20ref%29))
  (Utilities|Casting|CastToBP_FirstPersonCharacter OtherActor)
  (if (not (Variables|Default|GetBlockOpenDoor))
    (CallFunction|OpenDoor)
    (Variables|Default|SetBlockOpenDoor true)))

(event Custom|OpenDoor
  (bind _doorl (Variables|Default|GetDoorL))
  (bind _doorr (Variables|Default|GetDoorR))
  (bind _relativelocation (Variables|/Script/Engine.SceneComponent|GetRelativeLocation _doorl))
  (bind _relativelocation_2 (Variables|/Script/Engine.SceneComponent|GetRelativeLocation _doorr))
  (Audio|PlaySoundatLocation "/Game/Game/SoundDesign/Sound/SC_Door.SC_Door" (Transformation|GetActorLocation) "0, 0, 0" 1.0 (Class|GameplayStatics|GetGlobalTimeDilation) 0.5 0 0 0 0)
  (bind _outactors (Actor|GetAllActorsOfClass "/Game/Game/BluePrint/SoundDesing/BP_Musique.BP_Musique_C"))
  (bind _array_element (Utilities|Array|ForEachLoopwithBreak _outactors)
    (:LoopBody
      (if (== (Variables|/Script/Engine.AudioComponent|GetSound (Variables|/Game/Game/BluePrint/SoundDesing/BP_Musique.BP_Musique_C|GetMusique _array_element)) "/Game/Game/SoundDesign/Musique/SC_Lex.SC_Lex")
        (Default|LaucheMusique _array_element)
        (else
          (Default|StopMusique _array_element))))
    (:Completed
      (Utilities|FlowControl|Sequence
        (:then_0
          (Components|MoveComponentTo _doorl (Math|Vector|MakeVector (+ (.x _relativelocation) -5e+01) (.y _relativelocation) (.z _relativelocation)) (Variables|/Script/Engine.SceneComponent|GetRelativeRotation _doorl) false false 1.0 false))
        (:then_1
          (Components|MoveComponentTo _doorr (Math|Vector|MakeVector (+ (.x _relativelocation_2) 5e+01) (.y _relativelocation_2) (.z _relativelocation_2)) (Variables|/Script/Engine.SceneComponent|GetRelativeRotation _doorr) false false 1.0 false)))
      (Collision|SetCollisionResponsetoChannel (Variables|Default|GetDoorL) "ECC_GameTraceChannel2" "ECR_Ignore"))))

(event Custom|CloseDoor
  (bind _doorr (Variables|Default|GetDoorR))
  (bind _doorl (Variables|Default|GetDoorL))
  (bind _relativelocation (Variables|/Script/Engine.SceneComponent|GetRelativeLocation _doorr))
  (bind _relativelocation_2 (Variables|/Script/Engine.SceneComponent|GetRelativeLocation _doorl))
  (Collision|SetCollisionEnabled (Variables|Default|GetBox) "QueryAndPhysics")
  (Audio|PlaySoundatLocation "/Game/Game/SoundDesign/Sound/SC_Door.SC_Door" (Transformation|GetActorLocation) "0, 0, 0" 1.0 (Class|GameplayStatics|GetGlobalTimeDilation) 0.5 0 0 0 0)
  (Utilities|FlowControl|Sequence
    (:then_0
      (Components|MoveComponentTo _doorl (Math|Vector|MakeVector (+ (.x _relativelocation_2) 5e+01) (.y _relativelocation_2) (.z _relativelocation_2)) (Variables|/Script/Engine.SceneComponent|GetRelativeRotation _doorl) false false 1.0 false))
    (:then_1
      (Components|MoveComponentTo _doorr (Math|Vector|MakeVector (+ (.x _relativelocation) -5e+01) (.y _relativelocation) (.z _relativelocation)) (Variables|/Script/Engine.SceneComponent|GetRelativeRotation _doorr) false false 1.0 false)))
  (Collision|SetCollisionResponsetoChannel (Variables|Default|GetDoorL) "ECC_GameTraceChannel2" "ECR_Block"))

(event EventBeginPlay
  (Utilities|FlowControl|Delay 0.2)
  (bind _asbp_first_person_game_mode (Utilities|Casting|CastToBP_FirstPersonGameMode (Game|GetGameMode)))
  (Variables|Default|SetAs%20BP%20First%20Person%20Game%20Mode _asbp_first_person_game_mode))

(fn ConstructionScript)

(fn RemoveEnnemisfromList
  (params (EnnemieRef :type BP%20Ennemie%20Object%20Reference))
  (Utilities|Array|RemoveItem (Variables|Default|GetSameRoomEnnemisList) EnnemieRef)
  (if (<= (Utilities|Array|Length (Variables|Default|GetSameRoomEnnemisList)) 0)
    (CallFunction|OpenDoor)))